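; Climbing component for BP_LadderCharacter that handles ladders, horizontal ladders and climbable walls along the Y and Z axes.
; Each tick it polls every BP_ClimbVolume for overlap, attaches the character on up/down input in Flying mode, and switches to Falling on leaving.
; Directional input offsets the capsule directly, gated by line traces for surrounding obstacles.
; On moving ladders or walls, blocked traces push the character back or briefly disable the volume's collision.
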(event Custom|HeadAndFeetTrace
  ;[1 0.5998 0.226 1 30] LineTrace
  (if (and (Variables|Default|GetAttachedClimable) (not (Variables|Default|GetClimbThrough)))
    (CallFunction|RayTrace)))

(event Custom|MoveUp
  ;[0.45 1 0.3694 1 30] Movement
  (Utilities|AtTop?)
  (if (Math|Boolean|ANDBoolean (Variables|Default|GetAttachedClimable) (Utilities|Enum|Equal(Enum) (Variables|Default|GetKeyDirection) "NewEnumerator2") (not (Variables|Ditection|GetCeilingDetected)) (not (Variables|Default|GetHorizontal)))
    (Transformation|AddWorldOffset (Variables|/Script/Engine.Character|GetCapsuleComponent (Variables|Default|GetParent)) (Math|Vector|MakeVector 0.0 0.0 (Variables|Default|GetClimbSpeed)) false false)))

(event Custom|MoveRight
  ;[0.45 1 0.3694 1 30] Movement
  (if (Math|Boolean|ANDBoolean (Utilities|Enum|Equal(Enum) (Variables|Default|GetKeyDirection) "NewEnumerator1") (Variables|Default|GetAttachedClimable) (not (Variables|Ditection|GetRightDetected)) (not (Variables|Ditection|GetForwardDetected)))
    (Transformation|AddWorldOffset (Variables|/Script/Engine.Character|GetCapsuleComponent (Variables|Default|GetParent)) (Math|Vector|MakeVector 0.0 (* (Variables|Default|GetClimbSpeed) -1.0) 0.0) false false)
    (if (Variables|Default|GetHorizontal)
      (Transformation|SetWorldRotation (Variables|/Script/Engine.Character|GetCapsuleComponent (Variables|Default|GetParent)) "0,-90.000000, 0" false false))))

(event Custom|MoveDown
  (bind _parent (Variables|Default|GetParent))
  (bind _capsulecomponent (Variables|/Script/Engine.Character|GetCapsuleComponent _parent))
  ;[0.45 1 0.3694 1 30] Movement
  (if (Math|Boolean|ANDBoolean (Utilities|Enum|Equal(Enum) (Variables|Default|GetKeyDirection) "NewEnumerator3") (Variables|Default|GetAttachedClimable) (not (Variables|Ditection|GetFeetDownDetected)) (not (Variables|Default|GetHorizontal)))
    (if (Variables|Default|GetSlideDown)
      (Transformation|AddWorldOffset _capsulecomponent (Math|Vector|MakeVector 0.0 0.0 (* (Variables|Default|GetSlideSpeed) -1.0)) false false)
      (else
        (Transformation|AddWorldOffset _capsulecomponent (Math|Vector|MakeVector 0.0 0.0 (* (Variables|Default|GetClimbSpeed) -1.0)) false false)))))

(event Custom|VolumeCheck
  ;[1 0.376 0.9644 1 30] VolumeCheck
  (bind _outactors (Actor|GetAllActorsOfClass "/Game/2DLadders/BluePrints/Climbables/BP_ClimbVolume.BP_ClimbVolume_C"))
  (for (_array_element _array_index) _outactors
    (if (Variables|/Game/2DLadders/BluePrints/Climbables/BP_ClimbVolume.BP_ClimbVolume_C|GetOverlap _array_element)
      (Variables|Default|SetSectionNo _array_index)
      (Variables|Default|SetTop (Variables|/Game/2DLadders/BluePrints/Climbables/BP_ClimbVolume.BP_ClimbVolume_C|GetTop _array_element))
      (Variables|Ditection|SetOverLadder true)
      (bind _output_get (Variables|Default|SetClimbVolume _array_element))
      (Variables|Default|SetClimbType (Variables|/Game/2DLadders/BluePrints/Climbables/BP_ClimbVolume.BP_ClimbVolume_C|GetType _output_get))
      (Variables|Default|SetClimbTypeSub (Variables|/Game/2DLadders/BluePrints/Climbables/BP_ClimbVolume.BP_ClimbVolume_C|GetTypeSub _output_get))))
  (Utilities|FlowControl|Delay 0.01)
  (if (Variables|/Game/2DLadders/BluePrints/Climbables/BP_ClimbVolume.BP_ClimbVolume_C|GetOverlap (Utilities|Array|Get(acopy) _outactors (Variables|Default|GetSectionNo)))
    (goto _label Reset)
    (else
      (Utilities|FlowControl|DoOnce false :!label _label
        (:Completed
          (Variables|Ditection|SetOverLadder false)
          (Variables|Default|SetClimbThrough false)
          (Variables|Default|SetHorizontal false)
          (Default|DetachfromWall (Utilities|Array|Get(acopy) _outactors (Variables|Default|GetSectionNo)))
          (Default|DetachfromLadder (Utilities|Array|Get(acopy) _outactors (Variables|Default|GetSectionNo)))
          (Variables|Ditection|SetForwardDetected false)
          (Variables|Ditection|SetRightDetected false)
          (Variables|Ditection|SetLeftDetected false)
          (Variables|Ditection|SetFeetDownDetected false)
          (Variables|Ditection|SetCeilingDetected false))))))

(event Custom|Movement
  ;[0.45 1 0.3694 1 30] Movement
  (CallFunction|MoveUp)
  (CallFunction|MoveDown)
  (CallFunction|MoveLeft)
  (CallFunction|MoveRight)
  (CallFunction|Wallmoving))

(event Custom|wallmoving
  (bind _climbvolume (Variables|Default|GetClimbVolume))
  (bind _climbvolume_2 (Variables|Default|GetClimbVolume))
  (bind _ladderparent (Variables|/Game/2DLadders/BluePrints/Climbables/BP_ClimbVolume.BP_ClimbVolume_C|GetLadderParent _climbvolume))
  (bind _wallparent (Variables|/Game/2DLadders/BluePrints/Climbables/BP_ClimbVolume.BP_ClimbVolume_C|GetWallParent _climbvolume))
  (bind _movespeed (Variables|/Game/2DLadders/BluePrints/Climbables/BP_Ladder.BP_Ladder_C|GetMoveSpeed _ladderparent))
  (bind _movespeed_2 (Variables|/Game/2DLadders/BluePrints/Climbables/BP_ClimbWall.BP_ClimbWall_C|GetMoveSpeed _wallparent))
  (bind _returnvalue (* _movespeed_2 -1.0))
  ;[0.7039 0.4475 1 1 30] OnMovingWall
  (Utilities|IsValid _climbvolume
    (:Is%20Valid
      (switch Utilities|FlowControl|Switch|SwitchonEnum_climbable (Variables|/Game/2DLadders/BluePrints/Climbables/BP_ClimbVolume.BP_ClimbVolume_C|GetType _climbvolume)
        (:NewEnumerator0
          (Utilities|IsValid _ladderparent
            (:Is%20Valid
              (if (and (Variables|/Game/2DLadders/BluePrints/Climbables/BP_Ladder.BP_Ladder_C|GetMove _ladderparent) (Variables|Default|GetAttachedClimable))
                (switch Utilities|FlowControl|Switch|SwitchonEnum_direction (Variables|/Game/2DLadders/BluePrints/Climbables/BP_Ladder.BP_Ladder_C|GetDirection _ladderparent)
                  (:NewEnumerator0
                    (if (Variables|Ditection|GetRightDetected)
                      (Default|DetachfromLadder _climbvolume_2)
                      (Collision|SetCollisionEnabled (Variables|/Game/2DLadders/BluePrints/Climbables/BP_ClimbVolume.BP_ClimbVolume_C|GetBox (Variables|Default|GetClimbVolume)) "NoCollision" :!label _label)
                      (Utilities|FlowControl|Delay 0.1)
                      (Collision|SetCollisionEnabled (Variables|/Game/2DLadders/BluePrints/Climbables/BP_ClimbVolume.BP_ClimbVolume_C|GetBox (Variables|Default|GetClimbVolume)) "QueryAndPhysics")
                      (else
                        (Variables|Default|SetWallPush "0, 0, 0" :!label _label_2))))
                  (:NewEnumerator1
                    (if (Variables|Ditection|GetLeftDetected)
                      (Default|DetachfromLadder _climbvolume_2)
                      (goto _label)
                      (else
                        (goto _label_2))))
                  (:NewEnumerator2
                    (if (Variables|Ditection|GetCeilingDetected)
                      (Variables|Default|SetWallPush (Math|Vector|MakeVector 0.0 0.0 (* _movespeed -1.0)))
                      (else
                        (goto _label_2))))
                  (:NewEnumerator3
                    (if (Variables|Ditection|GetFeetDownDetected)
                      (Variables|Default|SetWallPush (Math|Vector|MakeVector 0.0 0.0 _movespeed))
                      (else
                        (goto _label_2)))))))))
        (:NewEnumerator3
          (Utilities|IsValid _wallparent
            (:Is%20Valid
              (if (and (Variables|/Game/2DLadders/BluePrints/Climbables/BP_ClimbWall.BP_ClimbWall_C|GetMoving _wallparent) (Variables|Default|GetAttachedClimable))
                (switch Utilities|FlowControl|Switch|SwitchonEnum_direction (Variables|/Game/2DLadders/BluePrints/Climbables/BP_ClimbWall.BP_ClimbWall_C|GetDirection _wallparent)
                  (:NewEnumerator0
                    (if (Variables|Ditection|GetRightDetected)
                      (Variables|Default|SetWallPush (Math|Vector|MakeVector 0.0 _movespeed_2 0.0))
                      (else
                        (Variables|Default|SetWallPush "0, 0, 0" :!label _label_3))))
                  (:NewEnumerator1
                    (if (Variables|Ditection|GetLeftDetected)
                      (Variables|Default|SetWallPush (Math|Vector|MakeVector 0.0 _returnvalue 0.0))
                      (else
                        (goto _label_3))))
                  (:NewEnumerator2
                    (if (Variables|Ditection|GetCeilingDetected)
                      (Variables|Default|SetWallPush (Math|Vector|MakeVector 0.0 0.0 _returnvalue))
                      (else
                        (goto _label_3))))
                  (:NewEnumerator3
                    (if (Variables|Ditection|GetFeetDownDetected)
                      (Variables|Default|SetWallPush (Math|Vector|MakeVector 0.0 0.0 _movespeed_2))
                      (if (> (Variables|Default|GetZpos) (Variables|Default|GetTop))
                        (Collision|SetCollisionEnabled (Variables|/Game/2DLadders/BluePrints/Climbables/BP_ClimbVolume.BP_ClimbVolume_C|GetBox (Variables|Default|GetClimbVolume)) "NoCollision")
                        (Utilities|FlowControl|Delay 0.1)
                        (Collision|SetCollisionEnabled (Variables|/Game/2DLadders/BluePrints/Climbables/BP_ClimbVolume.BP_ClimbVolume_C|GetBox (Variables|Default|GetClimbVolume)) "QueryAndPhysics"))
                      (else
                        (goto _label_3)))))))))))))

(event Custom|MoveLeft
  ;[0.45 1 0.3694 1 30] Movement
  (if (Math|Boolean|ANDBoolean (Variables|Default|GetAttachedClimable) (Utilities|Enum|Equal(Enum) (Variables|Default|GetKeyDirection) "NewEnumerator0") (not (Variables|Ditection|GetLeftDetected)) (not (Variables|Ditection|GetForwardDetected)))
    (Transformation|AddWorldOffset (Variables|/Script/Engine.Character|GetCapsuleComponent (Variables|Default|GetParent)) (Math|Vector|MakeVector 0.0 (Variables|Default|GetClimbSpeed) 0.0) false false)
    (if (Variables|Default|GetHorizontal)
      (Transformation|SetWorldRotation (Variables|/Script/Engine.Character|GetCapsuleComponent (Variables|Default|GetParent)) "0,90.000000, 0" false false))))

(event EventBeginPlay
  ;[1 0 0 1 50] Set To Your Character
  (bind _asbp_ladder_character (Utilities|Casting|CastToBP_LadderCharacter (Components|GetOwner)))
  (Variables|Default|SetParent _asbp_ladder_character))

(event EventTick
  (params (DeltaSeconds :type Float%20%28single-precision%29))
  (bind _keydirection (Variables|Default|GetKeyDirection))
  (bind _parent (Variables|Default|GetParent))
  (bind _climbvolume (Variables|Default|GetClimbVolume))
  (bind _horizontal (Variables|/Game/2DLadders/BluePrints/Climbables/BP_ClimbVolume.BP_ClimbVolume_C|GetHorizontal _climbvolume))
  ;[0.1995 0.5698 1 1 30] Comment
  (Variables|Default|SetZpos (.Z (Math|Vector|BreakVector (Transformation|GetWorldLocation (Variables|/Script/Engine.Character|GetCapsuleComponent _parent)))))
  (Transformation|AddWorldOffset (Variables|/Script/Engine.Actor|GetRootComponent _parent) (Variables|Default|GetWallPush) false false)
  (CallFunction|HeadandFeetTrace)
  (CallFunction|VolumeCheck)
  (CallFunction|Movement)
  (if (Variables|Ditection|GetOverLadder)
    (if (and (or (Utilities|Enum|Equal(Enum) _keydirection "NewEnumerator2") (Utilities|Enum|Equal(Enum) _keydirection "NewEnumerator3")) (or (and (<= (Variables|Default|GetZpos) (Variables|/Game/2DLadders/BluePrints/Climbables/BP_ClimbVolume.BP_ClimbVolume_C|GetTop _climbvolume)) (not _horizontal)) _horizontal))
      (CallFunction|AttachtoLadder)
      (goto _label Reset)
      (elif (Variables|Default|GetAttachedClimable)
        (CallFunction|AttachtoLadder)))
    (else
      (Variables|Default|SetAttachedClimable false)
      (Variables|Default|SetState "NewEnumerator0")
      (Utilities|FlowControl|DoOnce false :!label _label
        (:Completed
          (Pawn|Components|CharacterMovement|SetMovementMode (Variables|/Script/Engine.Character|GetCharacterMovement (Variables|Default|GetParent)) "MOVE_Falling" 0))))))

(fn AttachtoLadder
  (bind _parent (Variables|Default|GetParent))
  (bind _parent_2 (Variables|Default|GetParent))
  (bind _climbvolume (Variables|Default|GetClimbVolume))
  (bind _climbvolume_2 (Variables|Default|GetClimbVolume))
  (bind _rootcomponent (Variables|/Script/Engine.Actor|GetRootComponent _climbvolume))
  (bind _charactermovement (Variables|/Script/Engine.Character|GetCharacterMovement _parent_2))
  (bind _capsulecomponent (Variables|/Script/Engine.Character|GetCapsuleComponent _parent))
  (bind _returnvalue (Transformation|GetWorldLocation _capsulecomponent))
  (bind _returnvalue_2 (Transformation|GetWorldLocation _rootcomponent))
  (bind (_x _y) (Math|Vector|BreakVector _returnvalue))
  (bind (_x_2 _y_2 _z) (Math|Vector|BreakVector _returnvalue))
  (switch Utilities|FlowControl|Switch|SwitchonEnum_climbable (Variables|Default|GetClimbType)
    (:NewEnumerator0
      (if (Variables|Default|GetHorizontal)
        (if (Math|Float|InRange(Float) (.Yaw (Math|Rotator|BreakRotator (Transformation|GetWorldRotation _capsulecomponent))) 0.0 1.8e+02)
          (Variables|Default|Setrotation "0,90.000000, 0")
          (else
            (Variables|Default|Setrotation "0,-90.000000, 0")))
        (Transformation|SetWorldTransform _capsulecomponent (Math|Transform|MakeTransform (Math|Vector|MakeVector _x _y (- (.Z (Math|Vector|BreakVector _returnvalue_2)) 7e+01)) (Variables|Default|Getrotation)) false false)
        (Transformation|AttachActorToActor (Variables|Default|GetParent) (Variables|Default|GetClimbVolume) "None" "KeepWorld" "KeepWorld" "KeepWorld" true)
        (else
          (Transformation|SetWorldTransform _capsulecomponent (Math|Transform|MakeTransform (Math|Vector|MakeVector _x_2 (.Y (Math|Vector|BreakVector _returnvalue_2)) _z) "0.000000,180.000000,0.000000") false false)
          (Transformation|AttachActorToActor (Variables|Default|GetParent) (Variables|Default|GetClimbVolume) "None" "KeepWorld" "KeepRelative" "KeepRelative" true :!label _label))))
    (:NewEnumerator3
      (Transformation|SetWorldRotation _capsulecomponent "0,180.000000,0.000000" false false)
      (goto _label)))
  (Default|AttachedtoWall _climbvolume_2)
  (Default|AttachedtoLadder _climbvolume_2)
  (Pawn|Components|CharacterMovement|SetMovementMode _charactermovement "MOVE_Flying" 0)
  (Components|Movement|StopMovementImmediately _charactermovement)
  (Variables|Default|SetAttachedClimable true)
  (Variables|Default|SetState "NewEnumerator1"))

(fn RayTrace
  (bind _returnvalue (Utilities|VerticalRayTrace 5e+01 "None" "(R=1.000000,G=0.000000,B=0.783917,A=1.000000)"))
  (Variables|Ditection|SetCeilingDetected _returnvalue)
  (bind _returnvalue_2 (Utilities|VerticalRayTrace -7e+01 "None" "(R=0.000000,G=0.287186,B=1.000000,A=1.000000)"))
  (Variables|Ditection|SetFeetDownDetected _returnvalue_2)
  (bind _returnvalue_3 (Utilities|HorizontalRayTrace -1e+02 "None" "(R=0.000000,G=0.000000,B=0.000000,A=1.000000)" 0.0))
  (bind _returnvalue_4 (Utilities|HorizontalRayTrace -1e+02 "None" "(R=0.000000,G=0.000000,B=0.000000,A=1.000000)" -75.0))
  (bind _returnvalue_5 (Utilities|HorizontalRayTrace -1e+02 "None" "(R=0.000000,G=0.000000,B=0.000000,A=1.000000)" 75.0))
  (Variables|Ditection|SetLeftDetected (Math|Boolean|ORBoolean _returnvalue_3 _returnvalue_4 _returnvalue_5))
  (bind _returnvalue_6 (Utilities|HorizontalRayTrace 1e+01 "None" "(R=0.671875,G=0.671875,B=0.671875,A=1.000000)" 0.0))
  (bind _returnvalue_7 (Utilities|HorizontalRayTrace 1e+01 "None" "(R=0.671875,G=0.671875,B=0.671875,A=1.000000)" -75.0))
  (bind _returnvalue_8 (Utilities|HorizontalRayTrace 1e+01 "None" "(R=0.671875,G=0.671875,B=0.671875,A=1.000000)" 75.0))
  (Variables|Ditection|SetRightDetected (Math|Boolean|ORBoolean _returnvalue_6 _returnvalue_7 _returnvalue_8))
  (bind _returnvalue_9 (Utilities|ForwardRayTrace))
  (Variables|Ditection|SetForwardDetected _returnvalue_9))