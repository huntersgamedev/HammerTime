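; Climbable ladder or pole actor for 2.5D and Paper 2D platformers that can also move back and forth.
; The construction script builds it from repeated mesh sections, orients it by platformer type and computes the travel end point; Paper 2D Horizontal is unsupported.
; BeginPlay spawns and attaches a BP_ClimbVolume.
; When Move is set, Tick drives interpolated or constant-speed travel, flagging a delay at each turnaround.
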(event EventTick
  (params (DeltaSeconds :type Float%20%28single-precision%29))
  (bind _cube (Variables|Default|GetCube))
  (bind _returnvalue (Transformation|GetWorldLocation _cube))
  ;[1 1 1 1 30] Movement
  (Variables|Movement|SetCurrentPos _returnvalue)
  (if (Variables|Movement|GetMove)
    (Variables|Default|SetTopZ (.Z (Math|Vector|BreakVector _returnvalue)))
    (if (Variables|Movement|GetDelay)
      (Utilities|FlowControl|Delay (Variables|Movement|GetStopDelay))
      (Variables|Movement|SetDelay false)
      (else
        (CallFunction|Moving 0.0)))))

(event EventBeginPlay
  (bind (_sections _collision _p2dcollision _returnvalue) (Utilities|MakeTransforms))
  (bind _self self)
  ;[1 1 1 1 30] Comment
  (switch Utilities|FlowControl|Switch|SwitchonEnum_Perspective (Variables|Default|GetPlatformerType)
    (:NewEnumerator0
      (bind _returnvalue_2 (Game|SpawnActorfromClass "/Game/2DLadders/BluePrints/Climbables/BP_ClimbVolume.BP_ClimbVolume_C" _collision "Undefined" 0 _self 0 "NewEnumerator0" false 0))
      (bind _output_get (Variables|Default|SetVolume _returnvalue_2))
      (Transformation|AttachComponentToComponent (Variables|/Script/Engine.Actor|GetRootComponent _output_get) (Variables|Default|GetCube) "None" "KeepWorld" "KeepWorld" "KeepWorld" true))
    (:NewEnumerator1
      (bind _returnvalue_3 (Game|SpawnActorfromClass "/Game/2DLadders/BluePrints/Climbables/BP_ClimbVolume.BP_ClimbVolume_C" _p2dcollision "Undefined" 0 _self 0 "NewEnumerator0" false 0))
      (bind _output_get_2 (Variables|Default|SetVolume _returnvalue_3))
      (Transformation|AttachComponentToComponent (Variables|/Script/Engine.Actor|GetRootComponent _output_get_2) (Variables|Default|GetCube) "None" "KeepWorld" "KeepWorld" "KeepWorld" true))
    (:NewEnumerator5
      (bind _returnvalue_4 (Game|SpawnActorfromClass "/Game/2DLadders/BluePrints/Climbables/BP_ClimbVolume.BP_ClimbVolume_C" _returnvalue "Undefined" 0 _self 0 "NewEnumerator0" true 0))
      (bind _output_get_3 (Variables|Default|SetVolume _returnvalue_4))
      (Transformation|AttachComponentToComponent (Variables|/Script/Engine.Actor|GetRootComponent _output_get_3) (Variables|Default|GetCube) "None" "KeepWorld" "KeepWorld" "KeepWorld" true))))

(fn ConstructionScript
  (bind _output_get (Variables|Movement|SetStartPos (Transformation|GetWorldLocation (Variables|Default|GetCube))))
  (switch Utilities|FlowControl|Switch|SwitchonEnum_MoveMethod (Variables|Movement|GetMoveMetod)
    (:NewEnumerator0
      (Variables|Movement|SetMoveVectorts _output_get))
    (:NewEnumerator1
      _))
  (CallFunction|SetEndPos)
  (Utilities|Array|Clear (Variables|Default|GetMeshSections))
  (CallFunction|SetStartValues)
  (for _index (range 0 (- (Variables|Default|GetLength) 1))
    (CallFunction|Sections (.Sections (Utilities|MakeTransforms _index)) _index))
  (switch Utilities|FlowControl|Switch|SwitchonEnum_Perspective (Variables|Default|GetPlatformerType)
    (:NewEnumerator1
      (Transformation|SetWorldRotation (Variables|Default|GetCube) "0,90.000000, 0" false false))
    (:NewEnumerator5
      (Transformation|SetWorldRotation (Variables|Default|GetCube) (Math|Rotator|MakeRotator 0.0 9e+01 -9e+01) false false))
    (:NewEnumerator6
      (Utilities|FlowControl|DoOnce false
        (:Completed
          (Development|PrintString "Paper 2D Horizontal Not Supported as of now" true true "(R=1.000000,G=0.000000,B=0.090844,A=1.000000)"))))))

(fn SetStartValues
  (bind _cube (Variables|Default|GetCube))
  (bind _sectionsize (Variables|Default|GetSectionSize))
  (bind _returnvalue (Transformation|GetWorldLocation _cube))
  (bind _z (Math|Vector|BreakVector _returnvalue))
  (Variables|Default|SetTopZ (+ _z _sectionsize))
  (Variables|Default|SetBotZ (+ (- _z (* (Math|Conversions|ToFloat(Integer) (Variables|Default|GetLength)) _sectionsize)) _sectionsize))
  (Variables|Default|SetLength (Math|Integer|Clamp(Integer) (Variables|Default|GetLength) 1 50)))

(fn Sections
  (params (RelativeTransform :type Transform) (Index :type Integer))
  (bind _meshsections (Variables|Default|GetMeshSections))
  (bind _cube (Variables|Default|GetCube))
  (bind _output (Utilities|Array|Get(acopy) _meshsections Index))
  (switch Utilities|FlowControl|Switch|SwitchonEnum_climbType (Variables|Default|GetSubType)
    (:NewEnumerator0
      (Utilities|Array|SetArrayElem _meshsections Index "/Game/2DLadders/Props/SM_Metal_Ladder.SM_Metal_Ladder" true)
      (bind _returnvalue (AddComponent|AddStaticMeshComponent true RelativeTransform))
      (Transformation|AttachComponentToComponent _returnvalue _cube "None" "KeepWorld" "KeepWorld" "KeepWorld" true)
      (Components|StaticMesh|SetStaticMesh _returnvalue _output))
    (:NewEnumerator3
      (Utilities|Array|SetArrayElem _meshsections Index "/Game/2DLadders/Props/SM_pole.SM_pole" true)
      (bind _returnvalue_2 (AddComponent|AddStaticMeshComponent true RelativeTransform))
      (Transformation|AttachComponentToComponent _returnvalue_2 _cube "None" "KeepWorld" "KeepWorld" "KeepWorld" true)
      (Components|StaticMesh|SetStaticMesh _returnvalue_2 _output))))

(fn SetEndPos
  (bind _startpos (Variables|Movement|GetStartPos))
  (bind _startpos_2 (Variables|Movement|GetStartPos))
  (bind _startpos_3 (Variables|Movement|GetStartPos))
  (bind _startpos_4 (Variables|Movement|GetStartPos))
  (bind _startpos_5 (Variables|Movement|GetStartPos))
  (bind _startpos_6 (Variables|Movement|GetStartPos))
  (bind _startpos_7 (Variables|Movement|GetStartPos))
  (bind _startpos_8 (Variables|Movement|GetStartPos))
  (bind (_x _y _z) (Math|Vector|BreakVector _startpos_2))
  (bind (_x_2 _y_2 _z_2) (Math|Vector|BreakVector _startpos))
  (bind (_x_3 _y_3 _z_3) (Math|Vector|BreakVector _startpos_3))
  (bind (_x_4 _y_4 _z_4) (Math|Vector|BreakVector _startpos_4))
  (bind (_x_5 _y_5 _z_5) (Math|Vector|BreakVector _startpos_5))
  (bind (_x_6 _y_6 _z_6) (Math|Vector|BreakVector _startpos_6))
  (bind (_x_7 _y_7 _z_7) (Math|Vector|BreakVector _startpos_7))
  (bind (_x_8 _y_8 _z_8) (Math|Vector|BreakVector _startpos_8))
  (switch Utilities|FlowControl|Switch|SwitchonEnum_Perspective (Variables|Default|GetPlatformerType)
    (:NewEnumerator0
      (switch Utilities|FlowControl|Switch|SwitchonEnum_direction (Variables|Movement|GetDirection) :!label _label
        (:NewEnumerator0
          (Variables|Movement|SetEndPos (Math|Vector|MakeVector _x_7 (+ _y_7 (* (Variables|Movement|GetTilesToMove) (Variables|Default|GetSectionSize))) _z_7)))
        (:NewEnumerator1
          (Variables|Movement|SetEndPos (Math|Vector|MakeVector _x (- _y (* (Variables|Movement|GetTilesToMove) (Variables|Default|GetSectionSize))) _z)))
        (:NewEnumerator2
          (Variables|Movement|SetEndPos (Math|Vector|MakeVector _x_2 _y_2 (+ _z_2 (* (Variables|Movement|GetTilesToMove) (Variables|Default|GetSectionSize))))))
        (:NewEnumerator3
          (Variables|Movement|SetEndPos (Math|Vector|MakeVector _x_8 _y_8 (- _z_8 (* (Variables|Movement|GetTilesToMove) (Variables|Default|GetSectionSize)))))))
      (Variables|Movement|SetTragetPos (Variables|Movement|GetEndPos)))
    (:NewEnumerator1
      (switch Utilities|FlowControl|Switch|SwitchonEnum_direction (Variables|Movement|GetDirection)
        (:NewEnumerator0
          (bind _output_get (Variables|Movement|SetEndPos (Math|Vector|MakeVector (- _x_5 (* (Variables|Movement|GetTilesToMove) (Variables|Default|GetSectionSize))) _y_5 _z_5))))
        (:NewEnumerator1
          (Variables|Movement|SetEndPos (Math|Vector|MakeVector (+ _x_6 (* (Variables|Movement|GetTilesToMove) (Variables|Default|GetSectionSize))) _y_6 _z_6)))
        (:NewEnumerator2
          (Variables|Movement|SetEndPos (Math|Vector|MakeVector _x_3 _y_3 (+ _z_3 (* (Variables|Movement|GetTilesToMove) (Variables|Default|GetSectionSize))))))
        (:NewEnumerator3
          (Variables|Movement|SetEndPos (Math|Vector|MakeVector _x_4 _y_4 (- _z_4 (* (Variables|Movement|GetTilesToMove) (Variables|Default|GetSectionSize)))))))
      (Variables|Movement|SetTragetPos _output_get))
    (:NewEnumerator5
      (goto _label))))

(fn Moving
  (params (InputPin :type Float%20%28single-precision%29))
  (bind _platformertype (Variables|Default|GetPlatformerType))
  (bind _movespeed (Variables|Movement|GetMoveSpeed))
  (bind _movespeed_2 (Variables|Movement|GetMoveSpeed))
  (switch Utilities|FlowControl|Switch|SwitchonEnum_MoveMethod (Variables|Movement|GetMoveMetod)
    (:NewEnumerator0
      (Transformation|SetWorldLocation (Variables|Default|GetCube) (Variables|Movement|GetMoveVectorts) false false)
      (switch Utilities|FlowControl|Switch|SwitchonEnum_BackForward (Variables|Movement|GetForwardBack)
        (:NewEnumerator0
          (Variables|Movement|SetMoveVectorts (Math|Interpolation|VInterpTo (Variables|Movement|GetMoveVectorts) (Variables|Movement|GetEndPos) InputPin (Variables|Movement|GetMoveSpeed)))
          (if (Math|Vector|Equal(Vector) (Variables|Movement|GetMoveVectorts) (Variables|Movement|GetEndPos) 1e+01)
            (Variables|Movement|SetDelay true)
            (Variables|Movement|SetForwardBack "NewEnumerator1")))
        (:NewEnumerator1
          (Variables|Movement|SetMoveVectorts (Math|Interpolation|VInterpTo (Variables|Movement|GetMoveVectorts) (Variables|Movement|GetStartPos) InputPin (Variables|Movement|GetMoveSpeed)))
          (if (Math|Vector|Equal(Vector) (Variables|Movement|GetMoveVectorts) (Variables|Movement|GetStartPos) 1e+01)
            (Variables|Movement|SetDelay true)
            (Variables|Movement|SetForwardBack "NewEnumerator0")))))
    (:NewEnumerator1
      (Transformation|AddWorldOffset (Variables|Default|GetCube) (Variables|Movement|GetMoveVectorts) false false)
      (switch Utilities|FlowControl|Switch|SwitchonEnum_direction (Variables|Movement|GetDirection)
        (:NewEnumerator0
          (switch Utilities|FlowControl|Switch|SwitchonEnum_Perspective _platformertype
            (:NewEnumerator0
              (Variables|Movement|SetMoveVectorts (Math|Vector|MakeVector 0.0 _movespeed 0.0) :!label _label)
              (if (Math|Vector|Equal(Vector) (Variables|Movement|GetCurrentPos) (Variables|Movement|GetTragetPos) 1e+01)
                (Variables|Movement|SetDelay true)
                (Variables|Movement|SetDirection "NewEnumerator1")
                (switch Utilities|FlowControl|Switch|SwitchonEnum_BackForward (Variables|Movement|GetForwardBack) :!label _label_2
                  (:NewEnumerator0
                    (Variables|Movement|SetTragetPos (Variables|Movement|GetStartPos))
                    (Variables|Movement|SetForwardBack "NewEnumerator1"))
                  (:NewEnumerator1
                    (Variables|Movement|SetTragetPos (Variables|Movement|GetEndPos))
                    (Variables|Movement|SetForwardBack "NewEnumerator0")))))
            (:NewEnumerator1
              (Variables|Movement|SetMoveVectorts (Math|Vector|MakeVector _movespeed_2 0.0 0.0)))
            (:NewEnumerator5
              (goto _label))))
        (:NewEnumerator1
          (switch Utilities|FlowControl|Switch|SwitchonEnum_Perspective _platformertype
            (:NewEnumerator0
              (Variables|Movement|SetMoveVectorts (Math|Vector|MakeVector 0.0 (* _movespeed -1.0) 0.0) :!label _label_3))
            (:NewEnumerator1
              (Variables|Movement|SetMoveVectorts (Math|Vector|MakeVector (* _movespeed_2 -1.0) 0.0 0.0)))
            (:NewEnumerator5
              (goto _label_3)))
          (if (Math|Vector|Equal(Vector) (Variables|Movement|GetCurrentPos) (Variables|Movement|GetTragetPos) 1e+01)
            (Variables|Movement|SetDelay true)
            (Variables|Movement|SetDirection "NewEnumerator0")
            (goto _label_2)))
        (:NewEnumerator2
          (Variables|Movement|SetMoveVectorts (Math|Vector|MakeVector 0.0 0.0 (Variables|Movement|GetMoveSpeed)))
          (if (Math|Vector|Equal(Vector) (Variables|Movement|GetCurrentPos) (Variables|Movement|GetTragetPos) 1e+01)
            (Variables|Movement|SetDelay true)
            (Variables|Movement|SetDirection "NewEnumerator3")
            (goto _label_2)))
        (:NewEnumerator3
          (Variables|Movement|SetMoveVectorts (Math|Vector|MakeVector 0.0 0.0 (* (Variables|Movement|GetMoveSpeed) -1.0)))
          (if (Math|Vector|Equal(Vector) (Variables|Movement|GetCurrentPos) (Variables|Movement|GetTragetPos) 1e+01)
            (Variables|Movement|SetDelay true)
            (Variables|Movement|SetDirection "NewEnumerator2")
            (goto _label_2)))))))