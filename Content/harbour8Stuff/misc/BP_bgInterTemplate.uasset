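; Template trigger actor for a background switch, currently set up to open an assigned door in the level.
; When an actor implementing INTFACE_Interaction overlaps its Collider, a DoOnce gate lets it send OpenDoorMessage to ObjectToTrigger a single time.
; The construction script aligns the actor's root to the world X of the first BP_backgroundZone found, keeping its own Y and Z.
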(event OnComponentBeginOverlap(Collider)
  (params (OverlappedComponent :type Primitive%20Component%20Object%20Reference) (OtherActor :type Actor%20Object%20Reference) (OtherComp :type Primitive%20Component%20Object%20Reference) (OtherBodyIndex :type Integer) (bFromSweep :type Boolean) (SweepResult :type Hit%20Result%20Structure%20%28by%20ref%29))
  ;[1 1 1] if an actor with the tag inter overlaps then a it will open a specified door in the level. (This is more to serve as a template for a background switch)
  (if (Utilities|DoesObjectImplementInterface OtherActor "/Game/harbour8Stuff/Hittables/INTFACE_Interaction.INTFACE_Interaction_C")
    (Utilities|FlowControl|DoOnce false
      (:Completed
        (Class|INTFACEInteraction|OpenDoor(Message) (Variables|Default|GetObjectToTrigger))))))

(event EventBeginPlay)

(event Collision|EventActorBeginOverlap
  (params (OtherActor :type Actor%20Object%20Reference)))

(event EventTick
  (params (DeltaSeconds :type Float%20%28single-precision%29)))

(fn ConstructionScript
  (bind _defaultsceneroot (Variables|Default|GetDefaultSceneRoot))
  (bind _returnvalue (Transformation|GetWorldLocation _defaultsceneroot))
  (bind (_x _y _z) (Math|Vector|BreakVector _returnvalue))
  (bind _outactors (Actor|GetAllActorsOfClass "/Game/harbour8Stuff/backGround/BP_backgroundZone.BP_backgroundZone_C"))
  (Transformation|SetWorldLocation _defaultsceneroot (Math|Vector|MakeVector (.X (Math|Vector|BreakVector (Transformation|GetWorldLocation (Variables|/Game/harbour8Stuff/backGround/BP_backgroundZone.BP_backgroundZone_C|GetDefaultSceneRoot (Utilities|Array|Get(acopy) _outactors))))) _y _z) false false))