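; Base Blueprint for hittable objects that can be knocked into the level background by hammer attacks.
; HitResult triggers KnockIntoBackground only for a Heavy Attack with the Big Head hammer, ignoring its HammerNeeded input.
; A timeline slides the object along X to the background zone while a second track drives its height, then destroys it.
; SetBackGroundVariable caches the first BP_backgroundZone as that target but is not called here.
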(event Custom|KnockIntoBackground
  (Variables|Default|SetCurrentWorldLocation (Transformation|GetWorldLocation (Variables|Default|GetDefaultSceneRoot)))
  (bind (_direction _translatetobackground _inair) (Timeline|BackgroundKnockback PlayFromStart)
    (:Update
      ;[1 1 1] moves the enemy from current postion to the vector created previously
      (Transformation|SetWorldLocation (Variables|Default|GetDefaultSceneRoot) (Math|Vector|MakeVector (.X (Math|Vector|BreakVector (Math|Vector|Lerp(Vector) (Math|Vector|MakeVector (.X (Math|Vector|BreakVector (Variables|Default|GetCurrentWorldLocation))) (.Y (Math|Vector|BreakVector (Variables|Default|GetCurrentWorldLocation))) (.Z (Math|Vector|BreakVector (Variables|Default|GetCurrentWorldLocation)))) (Math|Vector|MakeVector (.X (Math|Vector|BreakVector (Transformation|GetWorldLocation (Variables|/Game/harbour8Stuff/backGround/BP_backgroundZone.BP_backgroundZone_C|GetDefaultSceneRoot (Variables|Default|GetLevelBackground))))) (.Y (Math|Vector|BreakVector (Variables|Default|GetCurrentWorldLocation))) (.Z (Math|Vector|BreakVector (Variables|Default|GetCurrentWorldLocation)))) _translatetobackground))) (.Y (Math|Vector|BreakVector (Math|Vector|Lerp(Vector) (Math|Vector|MakeVector (.X (Math|Vector|BreakVector (Variables|Default|GetCurrentWorldLocation))) (.Y (Math|Vector|BreakVector (Variables|Default|GetCurrentWorldLocation))) (.Z (Math|Vector|BreakVector (Variables|Default|GetCurrentWorldLocation)))) (Math|Vector|MakeVector (.X (Math|Vector|BreakVector (Transformation|GetWorldLocation (Variables|/Game/harbour8Stuff/backGround/BP_backgroundZone.BP_backgroundZone_C|GetDefaultSceneRoot (Variables|Default|GetLevelBackground))))) (.Y (Math|Vector|BreakVector (Variables|Default|GetCurrentWorldLocation))) (.Z (Math|Vector|BreakVector (Variables|Default|GetCurrentWorldLocation)))) _translatetobackground))) (Math|Float|Lerp (.Z (Math|Vector|BreakVector (Variables|Default|GetCurrentWorldLocation))) (+ (.Z (Math|Vector|BreakVector (Variables|Default|GetCurrentWorldLocation))) 2e+02) _inair)) false false))
    (:Finished
      (Actor|DestroyActor))))

(event EventBeginPlay)

(event Collision|EventActorBeginOverlap
  (params (OtherActor :type Actor%20Object%20Reference)))

(event EventTick
  (params (DeltaSeconds :type Float%20%28single-precision%29)))

(fn ConstructionScript)

(fn SetBackGroundVariable
  (bind _outactors (Actor|GetAllActorsOfClass "/Game/harbour8Stuff/backGround/BP_backgroundZone.BP_backgroundZone_C"))
  (Variables|Default|SetLevelBackground (Utilities|Array|Get(acopy) _outactors)))

(fn HitResult
  (params (AttackType :type STR%20Attack%20Type%20Structure) (HammerNeeded :type ENU_HammerType%20Enum :default "NewEnumerator0"))
  (bind (_attacktype _hammertype) (Utilities|Struct|BreakSTR_attackType AttackType))
  (switch Utilities|FlowControl|Switch|SwitchonENU_AttackType _attacktype
    (:NewEnumerator1
      (switch Utilities|FlowControl|Switch|SwitchonENU_HammerType _hammertype
        (:NewEnumerator1
          (CallFunction|KnockIntoBackground))))))