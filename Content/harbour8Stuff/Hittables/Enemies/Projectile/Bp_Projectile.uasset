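; Enemy projectile that moves by adding its ForceApplied offset to the sphere each tick, without sweeping.
; On overlap with BP_Henry, it reverses direction once if his repel field is active, otherwise it destroys itself.
; Once deflected, it sends a hit message with fixed damage to any BP_BaseAI it overlaps, then destroys itself.
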(event OnComponentBeginOverlap(Sphere)
  (params (OverlappedComponent :type Primitive%20Component%20Object%20Reference) (OtherActor :type Actor%20Object%20Reference) (OtherComp :type Primitive%20Component%20Object%20Reference) (OtherBodyIndex :type Integer) (bFromSweep :type Boolean) (SweepResult :type Hit%20Result%20Structure%20%28by%20ref%29))
  (Utilities|IsValid OtherActor
    (:Is%20Valid
      (bind _asbp_henry (Utilities|Casting|CastToBP_Henry OtherActor)
        (:then
          (if (and (Variables|/Game/Henry/BluePrints/BP_Henry.BP_Henry_C|GetRepelFeild _asbp_henry) (not (Variables|Default|GetAlreadyDeflected)))
            (Variables|Default|SetForceApplied (* (Variables|Default|GetForceApplied) -1.0))
            (Variables|Default|SetAlreadyDeflected true)
            (else
              (Actor|DestroyActor))))
        (:CastFailed
          (if (Variables|Default|GetAlreadyDeflected)
            (bind _asbp_base_ai (Utilities|Casting|CastToBP_BaseAI OtherActor))
            (Class|INTFACEInteraction|GotHit(Message) _asbp_base_ai 0.0 (Utilities|Struct|MakeSTR_attackType "NewEnumerator0" "NewEnumerator0") 5.0)
            (Actor|DestroyActor)))))))

(event EventBeginPlay)

(event Collision|EventActorBeginOverlap
  (params (OtherActor :type Actor%20Object%20Reference)))

(event EventTick
  (params (DeltaSeconds :type Float%20%28single-precision%29))
  (Transformation|AddWorldOffset (Variables|Default|GetSphere) (Variables|Default|GetForceApplied) false false))

(fn ConstructionScript)