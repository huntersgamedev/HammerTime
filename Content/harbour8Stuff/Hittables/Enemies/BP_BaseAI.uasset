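; Base enemy character that reacts to player hits with damage and knockback, destroying itself when health runs out.
; GotHit branches on attack and hammer type: melee hits launch it by player facing, while projectiles only deal damage.
; A heavy Big Head hit at low health instead runs a timeline that lifts it and lerps it along X to the level's BP_backgroundZone, then destroys it.
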(event Custom|KnockToBackground
  (Variables|Default|SetCurrentWorldLocation (Transformation|GetWorldLocation (Variables|Collision|GetCapsuleComponent)))
  (bind (_direction _translatetobackground _inair) (Timeline|BackgroundLaunch PlayFromStart)
    (:Update
      ;[1 1 1] moves the enemy from current postion to the vector created previously
      (Transformation|SetWorldLocation (Variables|Collision|GetCapsuleComponent) (Math|Vector|MakeVector (.X (Math|Vector|BreakVector (Math|Vector|Lerp(Vector) (Math|Vector|MakeVector (.X (Math|Vector|BreakVector (Variables|Default|GetCurrentWorldLocation))) (.Y (Math|Vector|BreakVector (Variables|Default|GetCurrentWorldLocation))) (.Z (Math|Vector|BreakVector (Variables|Default|GetCurrentWorldLocation)))) (Math|Vector|MakeVector (.X (Math|Vector|BreakVector (Transformation|GetWorldLocation (Variables|/Game/harbour8Stuff/backGround/BP_backgroundZone.BP_backgroundZone_C|GetDefaultSceneRoot (Variables|Default|GetlevelBackground))))) (.Y (Math|Vector|BreakVector (Variables|Default|GetCurrentWorldLocation))) (.Z (Math|Vector|BreakVector (Variables|Default|GetCurrentWorldLocation)))) _translatetobackground))) (.Y (Math|Vector|BreakVector (Math|Vector|Lerp(Vector) (Math|Vector|MakeVector (.X (Math|Vector|BreakVector (Variables|Default|GetCurrentWorldLocation))) (.Y (Math|Vector|BreakVector (Variables|Default|GetCurrentWorldLocation))) (.Z (Math|Vector|BreakVector (Variables|Default|GetCurrentWorldLocation)))) (Math|Vector|MakeVector (.X (Math|Vector|BreakVector (Transformation|GetWorldLocation (Variables|/Game/harbour8Stuff/backGround/BP_backgroundZone.BP_backgroundZone_C|GetDefaultSceneRoot (Variables|Default|GetlevelBackground))))) (.Y (Math|Vector|BreakVector (Variables|Default|GetCurrentWorldLocation))) (.Z (Math|Vector|BreakVector (Variables|Default|GetCurrentWorldLocation)))) _translatetobackground))) (Math|Float|Lerp (.Z (Math|Vector|BreakVector (Variables|Default|GetCurrentWorldLocation))) (+ (.Z (Math|Vector|BreakVector (Variables|Default|GetCurrentWorldLocation))) 2e+02) _inair)) false false))
    (:Finished
      (Actor|DestroyActor))))

(event EventBeginPlay
  (bind _outactors (Actor|GetAllActorsOfClass "/Game/harbour8Stuff/backGround/BP_backgroundZone.BP_backgroundZone_C"))
  (Variables|Default|SetLevelBackground (Utilities|Array|Get(acopy) _outactors)))

(event Collision|EventActorBeginOverlap
  (params (OtherActor :type Actor%20Object%20Reference)))

(event EventTick
  (params (DeltaSeconds :type Float%20%28single-precision%29)))

(event EventGotHit
  (params (PlayerFacing :type Float%20%28single-precision%29) (TypeOfHit :type STR%20Attack%20Type%20Structure) (Damage :type Float%20%28single-precision%29))
  (bind (_attacktype _hammertype) (Utilities|Struct|BreakSTR_attackType TypeOfHit))
  (Utilities|CalculateKnockBack PlayerFacing
    (:%20
      (Variables|Default|SetDamageReceived Damage)
      (switch Utilities|FlowControl|Switch|SwitchonENU_AttackType _attacktype
        (:NewEnumerator0
          (switch Utilities|FlowControl|Switch|SwitchonENU_HammerType _hammertype
            (:NewEnumerator0
              _)
            (:NewEnumerator1
              _)
            (:NewEnumerator2
              _)
            (:NewEnumerator3
              _)
            (:NewEnumerator4
              _)
            (:NewEnumerator5
              _))
          (CallFunction|DamageandKnockback))
        (:NewEnumerator1
          (switch Utilities|FlowControl|Switch|SwitchonENU_HammerType _hammertype
            (:NewEnumerator0
              (CallFunction|DamageandKnockback :!label _label))
            (:NewEnumerator1
              (if (< (/ (Variables|Default|GetHealth) (Variables|Default|GetMaxHealth)) 0.3)
                (CallFunction|KnocktoBackground)
                (else
                  (CallFunction|DamageandKnockback))))
            (:NewEnumerator2
              (goto _label))
            (:NewEnumerator3
              (goto _label))
            (:NewEnumerator4
              (goto _label))
            (:NewEnumerator5
              (goto _label))))
        (:NewEnumerator2
          (CallFunction|TakeAwayHealth (Variables|Default|GetDamageReceived)))))))

(fn ConstructionScript)

(fn TakeAwayHealth
  (params (Damage :type Float%20%28single-precision%29))
  (bind _output_get (Variables|Default|SetHealth (- (Variables|Default|GetHealth) Damage)))
  (Development|PrintString (Utilities|String|ToString(Float) _output_get))
  (if (<= _output_get 0.0)
    (Actor|DestroyActor)))

(fn DamageandKnockback
  (Character|LaunchCharacter (Variables|Default|GetNewLaunch) false false)
  (CallFunction|TakeAwayHealth (Variables|Default|GetDamageReceived)))