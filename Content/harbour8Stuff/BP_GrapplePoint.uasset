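; BP_GrapplePoint is a grapple anchor that tells the player character, BP_Henry, when it can be grappled.
; Each tick it traces on the Camera channel to Henry's capsule, checking for an unobstructed hit, range and hammer equip state.
; Results toggle Henry's CanGrapple and the PressQ prompt, also passing the point's location when enabled.
; Two DoOnce gates reset each other, so updates fire only on state changes.
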(event Custom|ResetUnabletograpple
  (Utilities|FlowControl|DoOnce false) ; enters at Reset
)

(event Custom|ResetEnableGrapple
  (bind _returnvalue (Game|GetPlayerCharacter 0))
  (bind _asbp_henry (Utilities|Casting|CastToBP_Henry _returnvalue))
  (Utilities|FlowControl|DoOnce false) ; enters at Reset
)

(event EventBeginPlay)

(event Collision|EventActorBeginOverlap
  (params (OtherActor :type Actor%20Object%20Reference)))

(event EventTick
  (params (DeltaSeconds :type Float%20%28single-precision%29))
  (bind _returnvalue (Game|GetPlayerCharacter 0))
  (bind _asbp_henry (Utilities|Casting|CastToBP_Henry _returnvalue))
  (bind _outhit (Collision|LineTraceByChannel (Transformation|GetWorldLocation (Variables|Default|GetDefaultSceneRoot)) (Transformation|GetWorldLocation (Variables|/Script/Engine.Character|GetCapsuleComponent (.AsBP%20Henry (Utilities|Casting|CastToBP_Henry (Game|GetPlayerCharacter 0))))) "TraceTypeQuery2" false (Utilities|Array|MakeArray self) "None"))
  (Utilities|IsValid (.hitactor _outhit)
    (:Is%20Valid
      (if (.bSuccess (Utilities|Casting|CastToBP_Henry (.hitactor _outhit)))
        (if (and (< (Transformation|GetDistanceTo (.AsBP%20Henry (Utilities|Casting|CastToBP_Henry (.hitactor _outhit)))) (Variables|Default|GetMaxDistanceFromGrapple)) (Utilities|Enum|Equal(Enum) (Variables|/Game/Henry/BluePrints/BP_Henry.BP_Henry_C|GetHammerEqipped (.AsBP%20Henry (Utilities|Casting|CastToBP_Henry (.hitactor _outhit)))) "NewEnumerator0"))
          (Utilities|FlowControl|DoOnce false
            (:Completed
              (Variables|/Game/Henry/BluePrints/BP_Henry.BP_Henry_C|SetCanGrapple _asbp_henry true)
              (Variables|/Game/Henry/BluePrints/BP_Henry.BP_Henry_C|SetGrappleLocation _asbp_henry (Transformation|GetWorldLocation (Variables|Default|GetDefaultSceneRoot)))
              (Rendering|SetVisibility (Variables|Default|GetPressQ) true false)
              (CallFunction|ResetUnabletograpple)))
          (else
            (Utilities|FlowControl|DoOnce false :!label _label
              (:Completed
                (Variables|/Game/Henry/BluePrints/BP_Henry.BP_Henry_C|SetCanGrapple (.AsBP%20Henry (Utilities|Casting|CastToBP_Henry (Game|GetPlayerCharacter 0))) false)
                (CallFunction|ResetEnableGrapple)
                (Rendering|SetVisibility (Variables|Default|GetPressQ) false false)))))
        (else
          (goto _label))))))

(fn ConstructionScript)