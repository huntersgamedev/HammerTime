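; BP_testEnemy is a test enemy for a side-scroller that gets knocked into the level background when hit.
; BeginPlay caches the player and the first background zone, and hides a test damage widget.
; HitEnemy shows player Strength as damage, awards XP, then runs a timeline lerping the enemy toward the zone's X with an upward offset, destroying it on finish.
; DamageEnemy subtracts HP but is not called here.
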(event EventBeginPlay
  ;[1 1 1] takes care of all neccesary casting and gets the level background
  (Rendering|SetVisibility (Variables|Default|GetTestingDamage) false false)
  (bind _outactors (Actor|GetAllActorsOfClass "/Game/harbour8Stuff/backGround/BP_backgroundZone.BP_backgroundZone_C"))
  (Variables|Default|SetlevelBackground (Utilities|Array|Get(acopy) _outactors))
  (bind _asside_scroller_character (Utilities|Casting|CastToSideScrollerCharacter (Game|GetPlayerCharacter 0)))
  (Variables|Default|SetgetPlayer _asside_scroller_character))

(event Collision|EventActorBeginOverlap
  (params (OtherActor :type Actor%20Object%20Reference)))

(event EventTick
  (params (DeltaSeconds :type Float%20%28single-precision%29)))

(event EventHitEnemy
  (bind _defaultsceneroot (Variables|Default|GetDefaultSceneRoot))
  (bind _getplayer (Variables|Default|GetgetPlayer))
  (bind _returnvalue (Transformation|GetWorldLocation _defaultsceneroot))
  ;[1 0.4041 0] TESTING updates damage widget and adds xp to player
  (CallFunction|UpdateTestDamage (Variables|/Game/harbour8Stuff/SideScrollerCharacter.SideScrollerCharacter_C|Getstrength _getplayer))
  (Default|AddXP _getplayer (Variables|Default|Getxp))
  ;[1 1 1] send enemy from current position to the background
  (bind (_direction _translatetobackground _inair) (Timeline|toBackground Play)
    (:Update
      ;;[1 1 1] moves the enemy from current postion to the vector created previously
      (Transformation|SetWorldLocation _defaultsceneroot (Math|Vector|Lerp(Vector) _returnvalue (Math|Vector|MakeVector (.X (Math|Vector|BreakVector (Transformation|GetWorldLocation (Variables|/Game/harbour8Stuff/backGround/BP_backgroundZone.BP_backgroundZone_C|GetBox (Variables|Default|GetlevelBackground))))) (.Y (Math|Vector|BreakVector _returnvalue)) 1.6e+02) _translatetobackground) false false)
      ;;[1 1 1] handles the up and down motion in the Z axsis
      (Transformation|AddWorldOffset _defaultsceneroot (Math|Vector|MakeVector 0.0 0.0 (Math|Float|Lerp 2e+01 2e+01 _inair)) false false))
    (:Finished
      (Actor|DestroyActor))))

(fn ConstructionScript)

(fn DamageEnemy
  (params (damage :type Float%20%28single-precision%29))
  (Variables|Default|SetHP (- (Variables|Default|GetHP) damage)))

(fn UpdateTestDamage
  (params (damage :type Float%20%28single-precision%29))
  (bind _testingdamage (Variables|Default|GetTestingDamage))
  ;[1 0.3502 0] TESTING displays the amount of damage the player is doing. This is to show that strength changes based on what state charecters in
  (Rendering|SetVisibility _testingdamage true false)
  (bind _aswid_damage_being_done (Utilities|Casting|CastToWID_damageBeingDone (UserInterface|GetUserWidgetObject _testingdamage)))
  (Variables|/Game/harbour8Stuff/testEnemies/WID_damageBeingDone.WID_damageBeingDone_C|SetdamageBeingDone _aswid_damage_being_done damage))