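; StickFigureCharacter is a player-controllable stick figure character that moves along world axes and turns its figure to match.
; MoveRight and MoveForward axis inputs feed movement along world X (inverted) and Y, independent of camera or control rotation.
; Each tick, the StickFigure component's relative rotation interpolates toward the yaw of the last movement input, easing back to a fixed -90 yaw when there is none.
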(event EventBeginPlay)

(event Collision|EventActorBeginOverlap
  (params (OtherActor :type Actor%20Object%20Reference)))

(event EventTick
  (params (DeltaSeconds :type Float%20%28single-precision%29))
  (bind _returnvalue (Class|Pawn|GetLastMovementInputVector))
  (bind _stickfigure (Variables|Default|GetStickFigure))
  (bind _relativerotation (Variables|/Script/Engine.SceneComponent|GetRelativeRotation _stickfigure))
  (if (Math|Vector|Equal(Vector) _returnvalue "0, 0, 0" 0.0001)
    (bind _output_get (Variables|Default|SetTargetRotation "0,-90.000000, 0"))
    (Transformation|SetRelativeRotation _stickfigure (Math|Interpolation|RInterpTo _relativerotation _output_get DeltaSeconds 1e+01) false false)
    (else
      (bind _output_get_2 (Variables|Default|SetTargetRotation (Math|Rotator|MakeRotator 0.0 0.0 (.Yaw (Math|Vector|GetYawPitchfromVector _returnvalue)))))
      (Transformation|SetRelativeRotation _stickfigure (Math|Interpolation|RInterpTo _relativerotation _output_get_2 DeltaSeconds 1e+01) false false))))

(event Input|AxisEvents|InputAxisMoveForward
  (params (AxisValue :type Float%20%28single-precision%29))
  (Pawn|Input|AddMovementInput (Math|Vector|MakeVector 0.0 AxisValue 0.0) 1.0 false))

(event Input|AxisEvents|InputAxisMoveRight
  (params (AxisValue :type Float%20%28single-precision%29))
  (Pawn|Input|AddMovementInput (* (Math|Vector|MakeVector AxisValue 0.0 0.0) -1.0) 1.0 false))

(fn ConstructionScript)