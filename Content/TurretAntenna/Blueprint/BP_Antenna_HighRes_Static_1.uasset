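; Poseable high-res antenna turret actor with a rotating base, engine, central mounts, four big and four small panel pairs, and four receptors.
; Exposed angles drive the central pivots, while alpha variables are lerped through collapsed graphs into panel and receptor roll limits.
; The Construction Script assigns mesh, glass and decal materials and applies the pose.
; Tick reapplies the same rotations every frame, so changes to those variables show at runtime.
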(event EventBeginPlay)

(event Collision|EventActorBeginOverlap
  (params (OtherActor :type Actor%20Object%20Reference)))

(event EventTick
  (params (DeltaSeconds :type Float%20%28single-precision%29))
  (bind _smallpanel_2 (Variables|RotationParameters|GetSmallPanel_2))
  (bind _bigpanel_1 (Variables|RotationParameters|GetBigPanel_1))
  (bind _bigpanel_2 (Variables|RotationParameters|GetBigPanel_2))
  (bind _bigpanel_3 (Variables|RotationParameters|GetBigPanel_3))
  (bind _bigpanel_4 (Variables|RotationParameters|GetBigPanel_4))
  (bind _smallpanel_1 (Variables|RotationParameters|GetSmallPanel_1))
  (bind _smallpanel_3 (Variables|RotationParameters|GetSmallPanel_3))
  (bind _smallpanel_4 (Variables|RotationParameters|GetSmallPanel_4))
  (bind _returnvalue (|CollapseGraph_0_2_2_2_2 _bigpanel_4))
  (bind _returnvalue_2 (|CollapseGraph_0_2_2 _bigpanel_2))
  (bind _returnvalue_3 (|CollapseGraph_0_2_2_2 _bigpanel_3))
  (bind _returnvalue_4 (|CollapseGraph_0_2 _bigpanel_1))
  ;[1 1 1] Central Rotations
  (Transformation|SetRelativeRotation (Variables|Default|GetbaseRot) (Math|Rotator|MakeRotator 0.0 0.0 (Variables|RotationParameters|GetBaseSupport)) false false)
  (Transformation|SetRelativeRotation (Variables|Default|GetEngineMovilRot) (Math|Rotator|MakeRotator (Variables|RotationParameters|GetEngine) 0.0 0.0) false false)
  (Transformation|SetRelativeRotation (Variables|Default|GetBaseCentralRot_1) (Math|Rotator|MakeRotator 0.0 (Variables|RotationParameters|GetBaseCentralAntenna) 0.0) false false)
  (Transformation|SetRelativeRotation (Variables|Default|GetBaseCentralRot_2) (Math|Rotator|MakeRotator 0.0 (Variables|RotationParameters|GetBaseCentralPanels) 0.0) false false)
  ;[1 1 1] Big Panels Rotation
  (Utilities|FlowControl|Sequence
    (:then_0
      (Transformation|SetRelativeRotation (Variables|Default|GetBigPanelInfMovil_1) (Math|Rotator|MakeRotator _returnvalue_4 0.0 0.0) false false)
      (Transformation|SetRelativeRotation (Variables|Default|GetBigPanelSupMovil_1) (Math|Rotator|MakeRotator _returnvalue_4 0.0 0.0) false false)
      ;[1 1 1] Small Panels Rotations
      (Utilities|FlowControl|Sequence
        (:then_0
          (Transformation|SetRelativeRotation (Variables|Default|GetSmallPanelInfMovil_1) (Math|Rotator|MakeRotator (|CollapseGraph_1_2 _smallpanel_1) 0.0 0.0) false false)
          (Transformation|SetRelativeRotation (Variables|Default|GetSmallPanelSupMovil_1) (Math|Rotator|MakeRotator (|CollapseGraph_2_2 _smallpanel_1) 0.0 0.0) false false)
          ;[1 1 1] Receptors Rotation
          (Utilities|FlowControl|Sequence
            (:then_0
              (Transformation|SetRelativeRotation (Variables|Default|GetReceptor_1) (Math|Rotator|MakeRotator (Math|Float|Lerp 1e+01 6e+01 (Variables|RotationParameters|GetReceptors)) 0.0 0.0) false false))))
        (:then_1
          (Transformation|SetRelativeRotation (Variables|Default|GetSmallPanelInfMovil_2) (Math|Rotator|MakeRotator (|CollapseGraph_3_2 _smallpanel_2) 0.0 0.0) false false)
          (Transformation|SetRelativeRotation (Variables|Default|GetSmallPanelSupMovil_2) (Math|Rotator|MakeRotator (|CollapseGraph_4_2 _smallpanel_2) 0.0 0.0) false false))
        (:then_2
          (Transformation|SetRelativeRotation (Variables|Default|GetSmallPanelInfMovil_3) (Math|Rotator|MakeRotator (|CollapseGraph_5_2 _smallpanel_3) 0.0 0.0) false false)
          (Transformation|SetRelativeRotation (Variables|Default|GetSmallPanelSupMovil_3) (Math|Rotator|MakeRotator (|CollapseGraph_6_2 _smallpanel_3) 0.0 0.0) false false))
        (:then_3
          (Transformation|SetRelativeRotation (Variables|Default|GetSmallPanelInfMovil_4) (Math|Rotator|MakeRotator (|CollapseGraph_7_2 _smallpanel_4) 0.0 0.0) false false)
          (Transformation|SetRelativeRotation (Variables|Default|GetSmallPanelSupMovil_4) (Math|Rotator|MakeRotator (|CollapseGraph_8_2 _smallpanel_4) 0.0 0.0) false false))))
    (:then_1
      (Transformation|SetRelativeRotation (Variables|Default|GetBigPanelInfMovil_2) (Math|Rotator|MakeRotator _returnvalue_2 0.0 0.0) false false)
      (Transformation|SetRelativeRotation (Variables|Default|GetBigPanelSupMovil_2) (Math|Rotator|MakeRotator _returnvalue_2 0.0 0.0) false false))
    (:then_2
      (Transformation|SetRelativeRotation (Variables|Default|GetBigPanelInfMovil_3) (Math|Rotator|MakeRotator _returnvalue_3 0.0 0.0) false false)
      (Transformation|SetRelativeRotation (Variables|Default|GetBigPanelSupMovil_3) (Math|Rotator|MakeRotator _returnvalue_3 0.0 0.0) false false))
    (:then_3
      (Transformation|SetRelativeRotation (Variables|Default|GetBigPanelInfMovil_4) (Math|Rotator|MakeRotator _returnvalue 0.0 0.0) false false)
      (Transformation|SetRelativeRotation (Variables|Default|GetBigPanelSupMovil_4) (Math|Rotator|MakeRotator _returnvalue 0.0 0.0) false false))))

(fn ConstructionScript
  (bind _smallpanel_2 (Variables|RotationParameters|GetSmallPanel_2))
  (bind _bigpanel_1 (Variables|RotationParameters|GetBigPanel_1))
  (bind _bigpanel_2 (Variables|RotationParameters|GetBigPanel_2))
  (bind _bigpanel_3 (Variables|RotationParameters|GetBigPanel_3))
  (bind _bigpanel_4 (Variables|RotationParameters|GetBigPanel_4))
  (bind _smallpanel_1 (Variables|RotationParameters|GetSmallPanel_1))
  (bind _smallpanel_3 (Variables|RotationParameters|GetSmallPanel_3))
  (bind _smallpanel_4 (Variables|RotationParameters|GetSmallPanel_4))
  (bind _returnvalue (|CollapseGraph_0_2_2_2 _bigpanel_4))
  (bind _returnvalue_2 (|CollapseGraph_0_2 _bigpanel_2))
  (bind _returnvalue_3 (|CollapseGraph_0_2_2 _bigpanel_3))
  (bind _returnvalue_4 (|CollapseGraph_0 _bigpanel_1))
  ;[1 1 1] Setting Materials
  (Rendering|Material|SetMaterial (Variables|Default|GetbaseTurret01) 0 (Variables|Default|GetM_Base))
  (Rendering|Material|SetMaterial (Variables|Default|GetbaseRot) 0 (Variables|Default|GetM_Antenna))
  (Rendering|Material|SetMaterial (Variables|Default|GetSmallPanelSupMovil_1) 1 (Variables|Default|GetM_Glass))
  ;[1 1 1] Decals Material
  (Rendering|Components|Decal|SetDecalMaterial (Variables|Default|GetBase_decal_1) (Variables|Default|GetM_DecalBase))
  (Rendering|Components|Decal|SetDecalMaterial (Variables|Default|GetBaseAntenna_decal_3) (Variables|Default|GetM_DecalAntennaBase))
  (Rendering|Components|Decal|SetDecalMaterial (Variables|Default|GetBaseReceptor_decal_3) (Variables|Default|GetM_DecalBaseReceptor))
  ;[1 1 1] Central Rotations
  (Transformation|SetRelativeRotation (Variables|Default|GetbaseRot) (Math|Rotator|MakeRotator 0.0 0.0 (Variables|RotationParameters|GetBaseSupport)) false false)
  (Transformation|SetRelativeRotation (Variables|Default|GetEngineMovilRot) (Math|Rotator|MakeRotator (Variables|RotationParameters|GetEngine) 0.0 0.0) false false)
  (Transformation|SetRelativeRotation (Variables|Default|GetBaseCentralRot_1) (Math|Rotator|MakeRotator 0.0 (Variables|RotationParameters|GetBaseCentralAntenna) 0.0) false false)
  (Transformation|SetRelativeRotation (Variables|Default|GetBaseCentralRot_2) (Math|Rotator|MakeRotator 0.0 (Variables|RotationParameters|GetBaseCentralPanels) 0.0) false false)
  ;[1 1 1] Big Panels Rotation
  (Utilities|FlowControl|Sequence
    (:then_0
      (Transformation|SetRelativeRotation (Variables|Default|GetBigPanelInfMovil_1) (Math|Rotator|MakeRotator _returnvalue_4 0.0 0.0) false false)
      (Transformation|SetRelativeRotation (Variables|Default|GetBigPanelSupMovil_1) (Math|Rotator|MakeRotator _returnvalue_4 0.0 0.0) false false)
      ;[1 1 1] Small Panels Rotations
      (Utilities|FlowControl|Sequence
        (:then_0
          (Transformation|SetRelativeRotation (Variables|Default|GetSmallPanelInfMovil_1) (Math|Rotator|MakeRotator (|CollapseGraph_1 _smallpanel_1) 0.0 0.0) false false)
          (Transformation|SetRelativeRotation (Variables|Default|GetSmallPanelSupMovil_1) (Math|Rotator|MakeRotator (|CollapseGraph_2 _smallpanel_1) 0.0 0.0) false false)
          ;[1 1 1] Receptors Rotation
          (Utilities|FlowControl|Sequence
            (:then_0
              (Transformation|SetRelativeRotation (Variables|Default|GetReceptor_1) (Math|Rotator|MakeRotator (Math|Float|Lerp 1e+01 6e+01 (Variables|RotationParameters|GetReceptors)) 0.0 0.0) false false))))
        (:then_1
          (Transformation|SetRelativeRotation (Variables|Default|GetSmallPanelInfMovil_2) (Math|Rotator|MakeRotator (|CollapseGraph_3 _smallpanel_2) 0.0 0.0) false false)
          (Transformation|SetRelativeRotation (Variables|Default|GetSmallPanelSupMovil_2) (Math|Rotator|MakeRotator (|CollapseGraph_4 _smallpanel_2) 0.0 0.0) false false))
        (:then_2
          (Transformation|SetRelativeRotation (Variables|Default|GetSmallPanelInfMovil_3) (Math|Rotator|MakeRotator (|CollapseGraph_5 _smallpanel_3) 0.0 0.0) false false)
          (Transformation|SetRelativeRotation (Variables|Default|GetSmallPanelSupMovil_3) (Math|Rotator|MakeRotator (|CollapseGraph_6 _smallpanel_3) 0.0 0.0) false false))
        (:then_3
          (Transformation|SetRelativeRotation (Variables|Default|GetSmallPanelInfMovil_4) (Math|Rotator|MakeRotator (|CollapseGraph_7 _smallpanel_4) 0.0 0.0) false false)
          (Transformation|SetRelativeRotation (Variables|Default|GetSmallPanelSupMovil_4) (Math|Rotator|MakeRotator (|CollapseGraph_8 _smallpanel_4) 0.0 0.0) false false))))
    (:then_1
      (Transformation|SetRelativeRotation (Variables|Default|GetBigPanelInfMovil_2) (Math|Rotator|MakeRotator _returnvalue_2 0.0 0.0) false false)
      (Transformation|SetRelativeRotation (Variables|Default|GetBigPanelSupMovil_2) (Math|Rotator|MakeRotator _returnvalue_2 0.0 0.0) false false))
    (:then_2
      (Transformation|SetRelativeRotation (Variables|Default|GetBigPanelInfMovil_3) (Math|Rotator|MakeRotator _returnvalue_3 0.0 0.0) false false)
      (Transformation|SetRelativeRotation (Variables|Default|GetBigPanelSupMovil_3) (Math|Rotator|MakeRotator _returnvalue_3 0.0 0.0) false false))
    (:then_3
      (Transformation|SetRelativeRotation (Variables|Default|GetBigPanelInfMovil_4) (Math|Rotator|MakeRotator _returnvalue 0.0 0.0) false false)
      (Transformation|SetRelativeRotation (Variables|Default|GetBigPanelSupMovil_4) (Math|Rotator|MakeRotator _returnvalue 0.0 0.0) false false))))