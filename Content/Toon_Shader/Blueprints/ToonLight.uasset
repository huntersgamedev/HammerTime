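; ToonLight is an actor that acts as a directional light source for toon shading by publishing its settings to Material Parameter Collections.
; LightChannel selects one of ten collections, which receives the negated forward vector, LightColor and LightBrightness as DirectLight parameters.
; An Arrow component is tinted to the light color.
; The update runs in the construction script, on BeginPlay and every Tick, so rotation and property changes propagate continuously.
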(event EventBeginPlay
  (CallFunction|LightInit))

(event Collision|EventActorBeginOverlap
  (params (OtherActor :type Actor%20Object%20Reference)))

(event EventTick
  (params (DeltaSeconds :type Float%20%28single-precision%29))
  (CallFunction|LightInit))

(fn ConstructionScript
  (CallFunction|LightInit))

(fn ArrowColor
  (Components|Arrow|SetArrowColor(LinearColor) (Variables|Default|GetArrow) (Variables|LightProperties|GetLight%20Color)))

(fn LightInit
  (CallFunction|LightFunction)
  (CallFunction|ArrowColor))

(fn LightFunction
  (bind _light_channel (Variables|LightProperties|GetLight%20Channel))
  (bind _returnvalue (Utilities|Select :Index _light_channel :Option%200 "/Game/Toon_Shader/Blueprints/ToonLight_Sources/LightChannel_0.LightChannel_0" :Option%201 "/Game/Toon_Shader/Blueprints/ToonLight_Sources/LightChannel_1.LightChannel_1" :Option%202 "/Game/Toon_Shader/Blueprints/ToonLight_Sources/LightChannel_2.LightChannel_2" :Option%203 "/Game/Toon_Shader/Blueprints/ToonLight_Sources/LightChannel_3.LightChannel_3" :Option%204 "/Game/Toon_Shader/Blueprints/ToonLight_Sources/LightChannel_4.LightChannel_4" :Option%205 "/Game/Toon_Shader/Blueprints/ToonLight_Sources/LightChannel_5.LightChannel_5" :Option%206 "/Game/Toon_Shader/Blueprints/ToonLight_Sources/LightChannel_6.LightChannel_6" :Option%207 "/Game/Toon_Shader/Blueprints/ToonLight_Sources/LightChannel_7.LightChannel_7" :Option%208 "/Game/Toon_Shader/Blueprints/ToonLight_Sources/LightChannel_8.LightChannel_8" :Option%209 "/Game/Toon_Shader/Blueprints/ToonLight_Sources/LightChannel_9.LightChannel_9"))
  (Rendering|Material|SetVectorParameterValue _returnvalue (Utilities|String|StringToName "DirectLight") (Math|Conversions|ToLinearColor(Vector) (* (Math|Rotator|GetRotationXVector (Transformation|GetActorRotation)) -1.0)) :!class /Script/Engine.KismetMaterialLibrary)
  (Rendering|Material|SetVectorParameterValue _returnvalue (Utilities|String|StringToName "DirectLight_Color") (Variables|LightProperties|GetLight%20Color) :!class /Script/Engine.KismetMaterialLibrary)
  (Rendering|Material|SetScalarParameterValue _returnvalue (Utilities|String|StringToName "DirectLight_Brightness") (Variables|LightProperties|GetLight%20Brightness) :!class /Script/Engine.KismetMaterialLibrary))